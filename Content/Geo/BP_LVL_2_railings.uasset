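; Modular railing prop Blueprint for level geometry that offers several wood railing pieces, including straight, tile and corner variants, in one actor.
; The construction script maps a boolean per piece to the visibility of its mesh component, so each instance can show any combination.
; It also reassigns the 4x4 mesh on construction and sets the 50cm tile's visibility twice.
; The event graph holds no logic.
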(fn `UserConstructionScript`
  (`StaticMeshComponent.SetStaticMesh` (`self.Lvl_3_wood_railings_4x4`) "/Game/Geo/lvl_3/Lvl_3_wood_railings_4x4.Lvl_3_wood_railings_4x4")
  (`SceneComponent.SetVisibility` (`self.Lvl_3_wood_railings_2m`) (`self.railings_2m`) false)
  (`SceneComponent.SetVisibility` (`self.Lvl_3_wood_railings_1m_tile`) (`self.railings_1m_tile`) false)
  (`SceneComponent.SetVisibility` (`self.Lvl_3_wood_railings_50cm_tile`) (`self.railings_50_cm_tile`) false)
  (`SceneComponent.SetVisibility` (`self.Lvl_3_wood_railings_2x2`) (`self.railings_corner_2x2`) false)
  (`SceneComponent.SetVisibility` (`self.Lvl_3_wood_railings_1x1`) (`self.railings_corner_1x1`) false)
  (`SceneComponent.SetVisibility` (`self.Lvl_3_wood_railings_50cm_tile`) (`self.railings_50_cm_tile`) false)
  (`SceneComponent.SetVisibility` (`self.Lvl_3_wood_railings_4x4`) (`self.railings_4x4`) false)
  (`SceneComponent.SetVisibility` (`self.Lvl_3_wood_railings_corner_50cm`) (`self.railings_corner_50cm`) false))