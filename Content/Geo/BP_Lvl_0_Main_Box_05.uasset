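; Level 0 main box geometry Blueprint, variant 05, used as a modular piece for building the level.
; The construction script assigns the LVL_0_BOX_05 mesh to the main box component.
; Four corner components are shown or hidden individually through the Corner01 to Corner04 variables, so each placed instance can toggle its corners.
; The event graph holds only disabled default events, so there is no runtime logic.
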(fn `UserConstructionScript`
  (`StaticMeshComponent.SetStaticMesh` (`self.LVL_0_BOX_05`) "/Game/Geo/00_Main_Boxes/LVL_0_BOX_05.LVL_0_BOX_05")
  (`SceneComponent.SetVisibility` (`self.LVL_0_Box_Corner_01`) (`self.Corner 01`) false)
  (`SceneComponent.SetVisibility` (`self.LVL_0_Box_Corners_02`) (`self.Corner 02`) false)
  (`SceneComponent.SetVisibility` (`self.LVL_0_Box_Corners_03`) (`self.Corner 03`) false)
  (`SceneComponent.SetVisibility` (`self.LVL_0_Box_Corners_04`) (`self.Corner 04`) false))