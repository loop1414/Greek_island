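; Modular level-geometry Blueprint for a balcony wall piece.
; The Construction Script assigns the base wall mesh, then toggles visibility of the base, door, window, three balcony options and long stairs from boolean variables.
; Each toggle affects only its own component, so variants are configured per instance without runtime logic; the event graph is empty.
; Despite the LVL_2 asset name, the components and mesh use LVL3 naming.
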(fn `UserConstructionScript`
  (`StaticMeshComponent.SetStaticMesh` (`self.LVL_3_Wall_Balconie_Base`) "/Game/Geo/lvl_3/LVL_3_Wall_Balconie_Base.LVL_3_Wall_Balconie_Base")
  (`SceneComponent.SetVisibility` (`self.LVL_3_Wall_Balconie_Base`) (`self.Wall_Balconie_Base`) false)
  (`SceneComponent.SetVisibility` (`self.LVL_3_Wall_Balconie_Door`) (`self.Wall_Balconie_Door`) false)
  (`SceneComponent.SetVisibility` (`self.LVL_3_Wall_Balconie_Window`) (`self.Wall_Balconie_Window`) false)
  (`SceneComponent.SetVisibility` (`self.Lvl_3_balconie_OP_01`) (`self.Balconie_OP_01`) false)
  (`SceneComponent.SetVisibility` (`self.Lvl_3_balconie_OP_02`) (`self.Balconie_OP_02`) false)
  (`SceneComponent.SetVisibility` (`self.Lvl_3_balconie_OP_03`) (`self.Balconie_OP_03`) false)
  (`SceneComponent.SetVisibility` (`self.LVL_3_Stairs_100_400`) (`self.stairs_long`) false))