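; Modular small balcony geometry Blueprint, configured entirely in the Construction Script with no active runtime logic.
; It sets the main mesh and toggles visibility of two base pieces, an enclosure and two roof pieces through per-part variables.
; The Blue variable, converted to an integer, selects which material slot receives the white boxes material instance on all six mesh components.
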(fn `UserConstructionScript`
  (`PrimitiveComponent.SetMaterial` (`self.LVL_3_Balconie_Small_main`) (`KismetMathLibrary.Conv_BoolToInt` (`self.Blue`)) "/Game/Textures/MI_Main_Boxes_White.MI_Main_Boxes_White")
  (`PrimitiveComponent.SetMaterial` (`self.LVL_3_Balconie_Small_Roof_02`) (`KismetMathLibrary.Conv_BoolToInt` (`self.Blue`)) "/Game/Textures/MI_Main_Boxes_White.MI_Main_Boxes_White")
  (`PrimitiveComponent.SetMaterial` (`self.LVL_3_Balconie_Small_roof_01`) (`KismetMathLibrary.Conv_BoolToInt` (`self.Blue`)) "/Game/Textures/MI_Main_Boxes_White.MI_Main_Boxes_White")
  (`PrimitiveComponent.SetMaterial` (`self.LVL_3_Balconie_Small_enclosure`) (`KismetMathLibrary.Conv_BoolToInt` (`self.Blue`)) "/Game/Textures/MI_Main_Boxes_White.MI_Main_Boxes_White")
  (`PrimitiveComponent.SetMaterial` (`self.LVL_3_Balconie_Small_Base_01`) (`KismetMathLibrary.Conv_BoolToInt` (`self.Blue`)) "/Game/Textures/MI_Main_Boxes_White.MI_Main_Boxes_White")
  (`PrimitiveComponent.SetMaterial` (`self.LVL_3_Balconie_Small_Base_02`) (`KismetMathLibrary.Conv_BoolToInt` (`self.Blue`)) "/Game/Textures/MI_Main_Boxes_White.MI_Main_Boxes_White")
  (`StaticMeshComponent.SetStaticMesh` (`self.LVL_3_Balconie_Small_main`) "/Game/Geo/Balconie_small/LVL_3_Balconie_Small_main.LVL_3_Balconie_Small_main")
  (`SceneComponent.SetVisibility` (`self.LVL_3_Balconie_Small_Base_01`) (`self.Balconie_Base_01`) false)
  (`SceneComponent.SetVisibility` (`self.LVL_3_Balconie_Small_Base_02`) (`self.Balconie_Base_02`) false)
  (`SceneComponent.SetVisibility` (`self.LVL_3_Balconie_Small_enclosure`) (`self.Balconie_Enclosure`) false)
  (`SceneComponent.SetVisibility` (`self.LVL_3_Balconie_Small_roof_01`) (`self.Balconie_roof_01`) false)
  (`SceneComponent.SetVisibility` (`self.LVL_3_Balconie_Small_Roof_02`) (`self.Balconie_roof_02`) false))