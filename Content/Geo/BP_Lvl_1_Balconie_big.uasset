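; BP_Lvl_1_Balconie_big is a configurable large balcony geometry piece built from LVL 3 balcony meshes.
; Its construction script assigns the white box material to all parts, using the Blue variable converted to an integer as the material slot index.
; It sets the main mesh and toggles enclosure, closed enclosure, two base and two roof parts through visibility variables.
; The event graph holds no active logic.
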(fn `UserConstructionScript`
  (`PrimitiveComponent.SetMaterial` (`self.LVL_3_Balconie_Big_Main_01`) (`KismetMathLibrary.Conv_BoolToInt` (`self.Blue`)) "/Game/Textures/MI_Main_Boxes_White.MI_Main_Boxes_White")
  (`PrimitiveComponent.SetMaterial` (`self.LVL_3_Balconie_Big_Base_01`) (`KismetMathLibrary.Conv_BoolToInt` (`self.Blue`)) "/Game/Textures/MI_Main_Boxes_White.MI_Main_Boxes_White")
  (`PrimitiveComponent.SetMaterial` (`self.LVL_3_Balconie_Big_Base_02`) (`KismetMathLibrary.Conv_BoolToInt` (`self.Blue`)) "/Game/Textures/MI_Main_Boxes_White.MI_Main_Boxes_White")
  (`PrimitiveComponent.SetMaterial` (`self.LVL_3_Balconie_Big_Roof_02`) (`KismetMathLibrary.Conv_BoolToInt` (`self.Blue`)) "/Game/Textures/MI_Main_Boxes_White.MI_Main_Boxes_White")
  (`PrimitiveComponent.SetMaterial` (`self.LVL_3_Balconie_Big_Roof_01`) (`KismetMathLibrary.Conv_BoolToInt` (`self.Blue`)) "/Game/Textures/MI_Main_Boxes_White.MI_Main_Boxes_White")
  (`PrimitiveComponent.SetMaterial` (`self.LVL_3_Balconie_Big_Closed_Enclosure`) (`KismetMathLibrary.Conv_BoolToInt` (`self.Blue`)) "/Game/Textures/MI_Main_Boxes_White.MI_Main_Boxes_White")
  (`PrimitiveComponent.SetMaterial` (`self.LVL_3_Balconie_Big_Enclosure`) (`KismetMathLibrary.Conv_BoolToInt` (`self.Blue`)) "/Game/Textures/MI_Main_Boxes_White.MI_Main_Boxes_White")
  (`StaticMeshComponent.SetStaticMesh` (`self.LVL_3_Balconie_Big_Main_01`) "/Game/Geo/Balconie_big/LVL_3_Balconie_Big_Main_01.LVL_3_Balconie_Big_Main_01")
  (`SceneComponent.SetVisibility` (`self.LVL_3_Balconie_Big_Enclosure`) (`self.Balconie_enclosure`) false)
  (`SceneComponent.SetVisibility` (`self.LVL_3_Balconie_Big_Closed_Enclosure`) (`self.Balconie_closed_enclosure`) false)
  (`SceneComponent.SetVisibility` (`self.LVL_3_Balconie_Big_Base_01`) (`self.Balconie_Base_01`) false)
  (`SceneComponent.SetVisibility` (`self.LVL_3_Balconie_Big_Base_02`) (`self.Balconie_base_02`) false)
  (`SceneComponent.SetVisibility` (`self.LVL_3_Balconie_Big_Roof_01`) (`self.Balconie_Roof_01`) false)
  (`SceneComponent.SetVisibility` (`self.LVL_3_Balconie_Big_Roof_02`) (`self.Balconie_Roof_02`) false))